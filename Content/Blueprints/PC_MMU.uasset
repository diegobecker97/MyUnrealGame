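; Player controller that flies BP_Player's MMU with six degrees of freedom through Enhanced Input.
; BeginPlay adds IMC_MMU and caches the pawn's MMU and left wrist pivots.
; Yaw and pitch rotate the MMU pivot about its own axes, roll adds relative rotation, and movement offsets it per trigger without delta-time scaling, with boost multiplying speed.
; Movement also tilts the wrist within clamped limits, resetting it on release.
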(event `self.ReceiveBeginPlay`
  ; Enable Inputs
  (`EnhancedInputSubsystemInterface.AddMappingContext` (pcsubsystem `EnhancedInputLocalPlayerSubsystem` (`GameplayStatics.GetPlayerController` 0)) "/Game/Input/IMC_MMU.IMC_MMU" 0 (struct))
  ; Set MMU Pivot
  (bind _asbp_player (cast `/Game/Blueprints/BP_Player` (`self.K2_GetPawn`)))
  (set `self.MMU_Pivot` (`/Game/Blueprints/BP_Player.MMU_Pivot` _asbp_player))
  ; Set wrist pivot
  (bind _asbp_player_2 (cast `/Game/Blueprints/BP_Player` (`self.K2_GetPawn`)))
  (set `self.LWrist_Pivot` (`/Game/Blueprints/BP_Player.LWrist_Pivot` _asbp_player_2)))

(event `EnhancedInput|/Game/Input/IA_Boost`
  (params (ActionValue :type Boolean) (ElapsedSeconds :type "Float (double-precision)") (TriggeredSeconds :type "Float (double-precision)") (InputAction :type "InputAction Object Reference" :default "/Game/Input/IA_Boost.IA_Boost"))
  ; Boost
  (:`Triggered`
    (set `self.CurrentSpeed` (* (`self.MoveSpeed`) (`self.BoostSpeed`))))
  (:`Completed`
    (set `self.CurrentSpeed` (`self.MoveSpeed`))))

(event `EnhancedInput|/Game/Input/IA_Yaw`
  (params (ActionValue :type "Float (double-precision)") (ElapsedSeconds :type "Float (double-precision)") (TriggeredSeconds :type "Float (double-precision)") (InputAction :type "InputAction Object Reference" :default "/Game/Input/IA_Yaw.IA_Yaw"))
  (bind _mmu_pivot (`self.MMU_Pivot`))
  ; Mouse X Yaw
  (:`Triggered`
    (`SceneComponent.K2_AddWorldRotation` _mmu_pivot (`KismetMathLibrary.RotatorFromAxisAndAngle` (`SceneComponent.GetUpVector` _mmu_pivot) ActionValue) false false)))

(event `EnhancedInput|/Game/Input/IA_Pitch`
  (params (ActionValue :type "Float (double-precision)") (ElapsedSeconds :type "Float (double-precision)") (TriggeredSeconds :type "Float (double-precision)") (InputAction :type "InputAction Object Reference" :default "/Game/Input/IA_Pitch.IA_Pitch"))
  (bind _mmu_pivot (`self.MMU_Pivot`))
  ; Mouse Y Pitch
  (:`Triggered`
    (`SceneComponent.K2_AddWorldRotation` _mmu_pivot (`KismetMathLibrary.RotatorFromAxisAndAngle` (* (`SceneComponent.GetRightVector` _mmu_pivot) (-1.0 -1.0 -1.0)) ActionValue) false false)))

(event `EnhancedInput|/Game/Input/IA_Roll`
  (params (ActionValue :type Boolean) (ElapsedSeconds :type "Float (double-precision)") (TriggeredSeconds :type "Float (double-precision)") (InputAction :type "InputAction Object Reference" :default "/Game/Input/IA_Roll.IA_Roll"))
  ; Roll
  (:`Triggered`
    (`SceneComponent.K2_AddRelativeRotation` (`self.MMU_Pivot`) (`KismetMathLibrary.MakeRotator` (`KismetMathLibrary.Conv_BoolToDouble` ActionValue)) false false)))

(event `EnhancedInput|/Game/Input/IA_Movement`
  (params (ActionValue :type "Vector Structure") (ElapsedSeconds :type "Float (double-precision)") (TriggeredSeconds :type "Float (double-precision)") (InputAction :type "InputAction Object Reference" :default "/Game/Input/IA_Movement.IA_Movement"))
  (bind _lwrist_pivot (`self.LWrist_Pivot`))
  (bind (_movement_x _movement_y) (`KismetMathLibrary.BreakVector` (`self.Movement`)))
  (bind (_movement_x_2 _movement_y_2 _movement_z) (`KismetMathLibrary.BreakVector` (`self.Movement`)))
  (bind (_returnvalue_roll _returnvalue_pitch) (`KismetMathLibrary.BreakRotator` (`KismetMathLibrary.MakeRotator` (`KismetMathLibrary.FClamp` (`KismetMathLibrary.NormalizeAxis` (+ (.roll (`SceneComponent.RelativeRotation` _lwrist_pivot)) _movement_y)) -10.0 10.0) (`KismetMathLibrary.FClamp` (`KismetMathLibrary.NormalizeAxis` (+ (.pitch (`SceneComponent.RelativeRotation` _lwrist_pivot)) (* _movement_x -1.0))) -10.0 10.0))))
  ; 3d Movement
  (:`Triggered`
    (set `self.Movement` ActionValue)
    (`SceneComponent.K2_AddRelativeLocation` (`self.MMU_Pivot`) (+ (* (`SceneComponent.GetForwardVector` (`self.MMU_Pivot`)) (`self.CurrentSpeed`) _movement_x_2) (* (`SceneComponent.GetRightVector` (`self.MMU_Pivot`)) (`self.CurrentSpeed`) _movement_y_2) (* (`SceneComponent.GetUpVector` (`self.MMU_Pivot`)) (`self.CurrentSpeed`) _movement_z)) false false)
    ; Wrist rotation
    (`SceneComponent.K2_SetRelativeRotation` _lwrist_pivot (`KismetMathLibrary.MakeRotator` _returnvalue_roll _returnvalue_pitch) false false))
  (:`Completed`
    (`self.ResetWristRotation`)))

(fn `ResetWristRotation`
  (`SceneComponent.K2_SetRelativeRotation` (`self.LWrist_Pivot`) (`KismetMathLibrary.MakeRotator` 0.0) false false))

(fn `UserConstructionScript`)