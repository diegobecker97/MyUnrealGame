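; BP_HealthComponent is an actor component that tracks its owner's health and reports changes and death.
; On BeginPlay it fills health to the maximum and binds to the owner's OnTakeAnyDamage event.
; Each hit subtracts clamped damage and broadcasts OnHealthChanged with the health fraction.
; At zero health it fires OnDeath unless IsDead is set, though nothing in this graph sets that flag.
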(event `self.ReceiveBeginPlay`
  (set `self.CurrentHealth` (`self.MaxHealth`))
  (add `Actor.OnTakeAnyDamage` (`self.GetOwner`) (delegate `HandleDamage`)))

(event `HandleDamage`
  (params (DamagedActor :type "Actor Object Reference") (Damage :type "Float (single-precision)") (DamageType :type "DamageType Object Reference") (InstigatedBy :type "Controller Object Reference") (DamageCauser :type "Actor Object Reference"))
  ; Take Dmg
  (set `self.CurrentHealth` (`KismetMathLibrary.FClamp` (- (`self.CurrentHealth`) Damage) 0.0 (`self.MaxHealth`)))
  ; Update percent
  (`self.OnHealthChanged` (/ (`self.CurrentHealth`) (`self.MaxHealth`)))
  ; dead check
  (if (and (<= (`self.CurrentHealth`) 0.0) (not (`self.IsDead`)))
    (`self.OnDeath`)))